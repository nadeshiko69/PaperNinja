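; Player Character Blueprint with Enhanced Input for camera look, camera-relative movement, sprinting and jumping.
; Sprint toggles max walk speed while held, and jumps from near standstill are briefly delayed, while moving jumps fire immediately.
; The first damage received, including from a force-kill input that damages itself, prints a death message and disables movement.
; Tick draws a debug arrow along the velocity.
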(event `self.ReceiveTick`
  (params (DeltaSeconds :type "Float (single-precision)"))
  (bind _returnvalue (`self.K2_GetActorLocation`))
  (`KismetSystemLibrary.DrawDebugArrow` _returnvalue (+ _returnvalue (`self.GetVelocity`))))

(event `self.ReceiveAnyDamage`
  (params (Damage :type "Float (single-precision)") (DamageType :type "DamageType Object Reference") (InstigatedBy :type "Controller Object Reference") (DamageCauser :type "Actor Object Reference"))
  (`/Engine/EditorBlueprintResources/StandardMacros.DoOnce` false
    (:`Completed`
      (`KismetSystemLibrary.PrintString` "died!")
      (`CharacterMovementComponent.DisableMovement` (`self.CharacterMovement`)) ; 移動を無効化
    )))

(event `EnhancedInput|/Game/Inputs/IA_Jump`
  (params (ActionValue :type Boolean) (ElapsedSeconds :type "Float (double-precision)") (TriggeredSeconds :type "Float (double-precision)") (InputAction :type "InputAction Object Reference" :default "/Game/Inputs/IA_Jump.IA_Jump"))
  (:`Triggered`
    (if (`self.CanJump`)
      (if (not (>= (`KismetMathLibrary.VSizeXY` (`self.GetVelocity`)) 10.0))
        (`KismetSystemLibrary.Delay` 0.2))
      (`self.Jump`))))

(event `EnhancedInput|/Game/Inputs/IA_Sprint`
  (params (ActionValue :type Boolean) (ElapsedSeconds :type "Float (double-precision)") (TriggeredSeconds :type "Float (double-precision)") (InputAction :type "InputAction Object Reference" :default "/Game/Inputs/IA_Sprint.IA_Sprint"))
  (bind _charactermovement (`self.CharacterMovement`))
  (:`Triggered`
    (set `CharacterMovementComponent.MaxWalkSpeed` 200.0 _charactermovement))
  (:`Completed`
    (set `CharacterMovementComponent.MaxWalkSpeed` 75.0 _charactermovement)))

(event `EnhancedInput|/Game/Inputs/IA_ForceKill`
  (params (ActionValue :type Boolean) (ElapsedSeconds :type "Float (double-precision)") (TriggeredSeconds :type "Float (double-precision)") (InputAction :type "InputAction Object Reference" :default "/Game/Inputs/IA_ForceKill.IA_ForceKill"))
  (:`Triggered`
    (`GameplayStatics.ApplyDamage` self 1.0 null self)))

(event `EnhancedInput|/Game/Inputs/IA_Look`
  (params (ActionValue :type "Vector2D Structure") (ElapsedSeconds :type "Float (double-precision)") (TriggeredSeconds :type "Float (double-precision)") (InputAction :type "InputAction Object Reference" :default "/Game/Inputs/IA_Look.IA_Look"))
  (:`Triggered`
    (`self.AddControllerYawInput` (`KismetMathLibrary.BreakVector2D` ActionValue))
    (`self.AddControllerPitchInput` (`.Y` (`KismetMathLibrary.BreakVector2D` ActionValue)))))

(event `EnhancedInput|/Game/Inputs/IA_Move`
  (params (ActionValue :type "Vector2D Structure") (ElapsedSeconds :type "Float (double-precision)") (TriggeredSeconds :type "Float (double-precision)") (InputAction :type "InputAction Object Reference" :default "/Game/Inputs/IA_Move.IA_Move"))
  (:`Triggered`
    (`self.AddMovementInput` (`KismetMathLibrary.Cross_VectorVector` (`SceneComponent.GetRightVector` (`self.Camera`)) (`KismetMathLibrary.Vector_Up`)) (`.Y` (`KismetMathLibrary.BreakVector2D` ActionValue))) ; 前後移動
    (`self.AddMovementInput` (`SceneComponent.GetRightVector` (`self.Camera`)) (`KismetMathLibrary.BreakVector2D` ActionValue)) ; 左右移動
  ))

(fn `UserConstructionScript`)